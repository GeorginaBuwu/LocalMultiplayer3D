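; BP_SharedCamera is a shared camera actor that follows the midpoint of a group of players.
; UpdateActivePlayers stores the Players array and sets IsInGame, which enables the follow logic in Tick.
; Each tick, it lerps its location toward the players' average location, using SpeedMovement as a fixed alpha, so smoothing depends on frame rate.
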(event `self.ReceiveTick`
  (params (DeltaSeconds :type "Float (single-precision)"))
  (if (`self.Is in Game`)
    (bind _output_get (set `self.prevPost` (`self.K2_GetActorLocation`)))
    (bind _returnvalue (`GameplayStatics.GetActorArrayAverageLocation` (`self.Players`)))
    (`self.K2_SetActorLocation` (`KismetMathLibrary.VLerp` _output_get _returnvalue (`self.SpeedMovement`)))))

(fn `UpdateActivePlayers`
  (params (Players :type "Array of Actor Object Reference"))
  (set `self.Players` Players)
  (set `self.Is in Game` true))

(fn `UserConstructionScript`)