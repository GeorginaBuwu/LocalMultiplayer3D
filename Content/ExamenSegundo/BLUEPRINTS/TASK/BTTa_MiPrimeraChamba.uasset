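; Behavior Tree task that plays a typing loop on BP_GODIN while randomly draining its hunger, bathroom or sleep stat.
; Every two seconds it lowers one stat until the one just lowered is 45 or below.
; It then clears that need's Blackboard key, sets Work, switches to the walk animation and finishes successfully.
; Debug prints trace each step, and an older TRABAJO-progress version of the loop remains unconnected.
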(event `self.ReceiveExecuteAI`
  (params (OwnerController :type "AIController Object Reference") (ControlledPawn :type "Pawn Object Reference"))
  (bind _returnvalue (`KismetMathLibrary.RandomInteger` 3))
  (bind _asbp_godin (cast `/Game/ExamenSegundo/BP_GODIN` ControlledPawn))
  (`KismetSystemLibrary.PrintString` (`KismetStringLibrary.Conv_IntToString` _returnvalue) :!label _label)
  (switch `int` _returnvalue
    (:`0`
      (bind _output_get (set `/Game/ExamenSegundo/BP_GODIN.HAMBRE` (- (`/Game/ExamenSegundo/BP_GODIN.HAMBRE` _asbp_godin) 8) _asbp_godin))
      (`KismetSystemLibrary.PrintString` "El hambre baja" true true (struct :`R` 1.0 :`G` 0.055672 :`A` 1.0))
      (`KismetSystemLibrary.PrintString` (`KismetStringLibrary.Conv_IntToString` _output_get) true true (struct :`R` 1.0 :`B` 0.012455 :`A` 1.0))
      (if (<= _output_get 45)
        (`BTFunctionLibrary.SetBlackboardValueAsBool` (`self.HAMBRE?`))
        (else
          (`SkeletalMeshComponent.PlayAnimation` (`Character.Mesh` _asbp_godin) "/Game/ExamenSegundo/MONO/ANIMACIONES/Typing.Typing" true :!label _label_2)
          (`KismetSystemLibrary.Delay` 2.0)
          (goto _label))))
    (:`1`
      (bind _output_get_2 (set `/Game/ExamenSegundo/BP_GODIN.BANIO` (- (`/Game/ExamenSegundo/BP_GODIN.BANIO` _asbp_godin) 4) _asbp_godin))
      (`KismetSystemLibrary.PrintString` "adios popo")
      (`KismetSystemLibrary.PrintString` (`KismetStringLibrary.Conv_IntToString` _output_get_2))
      (if (<= _output_get_2 45)
        (`BTFunctionLibrary.SetBlackboardValueAsBool` (`self.MEAR`))
        (else
          (goto _label_2))))
    (:`2`
      (bind _output_get_3 (set `/Game/ExamenSegundo/BP_GODIN.MIMIR` (- (`/Game/ExamenSegundo/BP_GODIN.MIMIR` _asbp_godin) 2) _asbp_godin))
      (`KismetSystemLibrary.PrintString` "MIMIR" true true (struct :`R` 0.963901 :`G` 1.0 :`A` 1.0))
      (`KismetSystemLibrary.PrintString` (`KismetStringLibrary.Conv_IntToString` _output_get_3) true true (struct :`R` 1.0 :`G` 0.926811 :`A` 1.0))
      (if (<= _output_get_3 45)
        (`BTFunctionLibrary.SetBlackboardValueAsBool` (`self.AMIMIR?`))
        (else
          (goto _label_2)))))
  (`SkeletalMeshComponent.PlayAnimation` (`Character.Mesh` _asbp_godin) "/Game/ExamenSegundo/MONO/ANIMACIONES/Standard_Walk__1_.Standard_Walk__1_" true)
  (`BTFunctionLibrary.SetBlackboardValueAsBool` (`self.work`) true)
  (`self.FinishExecute` true))