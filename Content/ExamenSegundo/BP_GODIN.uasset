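; BP_GODIN is an office-worker ("godín") Blueprint that exposes the world locations of its daily-routine spots: bed, bathroom, job, kitchen and laundry.
; Each getter validates an actor reference and returns its location, or logs or prints a Spanish fallback message when the reference is missing.
; The event graph and construction script are empty, so nothing in this Blueprint calls the getters or moves the actor.
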(fn `alacamita`
  (returns (NewParam :type "Vector Structure"))
  (bind _bedlocation (`self.BedLocation`)
    (:`then`
      (return (`self.K2_GetActorLocation` _bedlocation)))
    (:`else`
      (`KismetSystemLibrary.LogString` "Duermes en el piso, Las gatas no tienen cama"))))

(fn `BatterLocation`
  (returns (BatterVector :type "Vector Structure"))
  (bind _bannio (`self.BANNIO`)
    (:`then`
      (return (`self.K2_GetActorLocation` _bannio)))
    (:`else`
      (`KismetSystemLibrary.LogString` "nO HAY BAÑOOOOOO"))))

(fn `ChambaLocartion`
  (returns (Location :type "Vector Structure"))
  (bind _chambalocation (`self.ChambaLocation`)
    (:`then`
      (return (`self.K2_GetActorLocation` _chambalocation)))
    (:`else`
      (`KismetSystemLibrary.PrintString` "NO TIENE CHAMBA"))))

(fn `GETPOSITIONDINNER`
  (returns (Location :type "Vector Structure"))
  (bind _dinnerlocation (`self.DinnerLocation`)
    (:`then`
      (return (`self.K2_GetActorLocation` _dinnerlocation)))
    (:`else`
      (`KismetSystemLibrary.PrintString` "No se encuentra la cocina"))))

(fn `LavadoraLocation`
  (returns (Locattion :type "Vector Structure"))
  (bind _ropa (`self.Ropa`)
    (:`then`
      (return (`self.K2_GetActorLocation` _ropa)))
    (:`else`
      (`KismetSystemLibrary.PrintString` "RopaSucia"))))

(fn `UserConstructionScript`)