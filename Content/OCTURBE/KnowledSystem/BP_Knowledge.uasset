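; BP_Knowledge is an NPC character Blueprint that supplies movement and patrol helpers.
; It sets walk speed through the CharacterMovement component and exposes itself through GetNPC.
; GetNextPatrolPoint asks the PatrolPath for the location after the current spline index, stores the returned index and returns the target, printing a warning when the path is invalid.
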(fn `GetNextPatrolPoint`
  (returns (PatrolTarget :type "Vector Structure"))
  (bind _patrolpath (`self.PatrolPath`)
    (:`then`
      (bind (_newindex _targetlocation) (`/Game/OCTURBE/KnowledSystem/BP_PATROLSLINE.GetPointLocation` _patrolpath (+ (`self.CurrentSplinePosition`) 1)))
      (set `self.CurrentSplinePosition` _newindex)
      (return _targetlocation))
    (:`else`
      (`KismetSystemLibrary.PrintString` "Patrol path is not valid check BP"))))

(fn `GetNPC`
  (returns (NPC :type "/Game/OCTURBE/KnowledSystem/BP_Knowledge Object Reference"))
  (return self))

(fn `UpdateWalkSpeed`
  (params (`New Walk Speed` :type "Float (double-precision)"))
  (set `CharacterMovementComponent.MaxWalkSpeed` `New Walk Speed` (`self.CharacterMovement`)))

(fn `UserConstructionScript`)